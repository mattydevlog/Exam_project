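; BP_HPpickup is a health pickup actor that heals the player on touch.
; It caches the player character on BeginPlay and compares it against actors entering its Box overlap.
; On a match it prints a debug message, adds a fixed amount to BP_FirstPersonCharacter's Health with no clamp in this graph, then destroys itself.
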(event `self.ReceiveBeginPlay`
  ;[0.589 0.3577 1] Set player ref
  (set `self.PlayerREF` (`GameplayStatics.GetPlayerCharacter` 0)))

(event `self.Box.OnComponentBeginOverlap`
  (params (OverlappedComponent :type "PrimitiveComponent Object Reference") (OtherActor :type "Actor Object Reference") (OtherComp :type "PrimitiveComponent Object Reference") (OtherBodyIndex :type Integer) (bFromSweep :type Boolean) (SweepResult :type "HitResult Structure (by ref)"))
  ;[1 0.6244 0.5444] Pickup behavior
  (if (== OtherActor (`self.PlayerREF`))
    (`KismetSystemLibrary.PrintString` "HP pickup taken")
    (bind _asbp_first_person_character (cast `/Game/FirstPerson/Blueprints/BP_FirstPersonCharacter` (`GameplayStatics.GetPlayerCharacter` 0)))
    (set `/Game/FirstPerson/Blueprints/BP_FirstPersonCharacter.health` (+ (`/Game/FirstPerson/Blueprints/BP_FirstPersonCharacter.health` _asbp_first_person_character) 5) _asbp_first_person_character)
    (`self.K2_DestroyActor`)))

(fn `UserConstructionScript`)