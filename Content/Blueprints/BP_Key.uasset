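; BP_Key is a key pickup actor for the first-person player.
; It caches the player character on BeginPlay and compares it against actors that begin overlapping its Box component.
; On a match it prints a debug message, sets the BhasKey flag on BP_FirstPersonCharacter and destroys itself.
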(event `self.ReceiveBeginPlay`
  (set `self.PlayerREF` (`GameplayStatics.GetPlayerCharacter` 0)))

(event `self.Box.OnComponentBeginOverlap`
  (params (OverlappedComponent :type "PrimitiveComponent Object Reference") (OtherActor :type "Actor Object Reference") (OtherComp :type "PrimitiveComponent Object Reference") (OtherBodyIndex :type Integer) (bFromSweep :type Boolean) (SweepResult :type "HitResult Structure (by ref)"))
  (if (== OtherActor (`self.PlayerREF`))
    (`KismetSystemLibrary.PrintString` "key picked up")
    (bind _asbp_first_person_character (cast `/Game/FirstPerson/Blueprints/BP_FirstPersonCharacter` (`GameplayStatics.GetPlayerCharacter` 0)))
    (set `/Game/FirstPerson/Blueprints/BP_FirstPersonCharacter.bhasKey` true _asbp_first_person_character)
    (`self.K2_DestroyActor`)))

(fn `UserConstructionScript`)