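; BP_Enemy1 is a shooting enemy that moves to the player when PawnSensing sees a pawn.
; While alive and moving, Tick runs a delayed forward line trace with a Niagara effect, but applies no damage.
; TakeDamage lowers HP and clears IsAlive at zero, after which Tick destroys the actor.
; A separate Death event adds an emitter before destroying it; the hit-reaction chain calling DamageVFX is disconnected.
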(event `self.PawnSensing.OnSeePawn`
  (params (Pawn :type "Pawn Object Reference"))
  ;[1 0.1593 0.9455] AI movement
  (bind _asbp_first_person_character (cast `/Game/FirstPerson/Blueprints/BP_FirstPersonCharacter` (`GameplayStatics.GetPlayerCharacter` 0)))
  (`|AIMoveTo` Pawn (0.0 0.0 0.0) _asbp_first_person_character
    (:`then`
      (set `self.isMoving` true))
    (:`OnFail`
      (set `self.isMoving` false))))

(event `Damage VFX`
  ;[1 1 1] VFX damage on player attack
  (`NiagaraFunctionLibrary.SpawnSystemAtLocation` null (`SceneComponent.K2_GetComponentLocation` (`self.Sphere`))))

(event `TakeDamage`
  ;[0.3545 1 0.2159] Taking damage
  (bind _output_get (set `self.HP1` (- (`self.HP1`) 1.0)))
  (if (<= _output_get 0.0)
    (set `self.isAlive` false)))

(event `Death`
  ;[0.04746 1 0.9103] Death state
  (if (not (`self.isAlive`))
    (`GameplayStatics.SpawnEmitterAtLocation` null (`SceneComponent.K2_GetComponentLocation` (`self.Sphere1`)))
    (`self.K2_DestroyActor`)))

(event `self.ReceiveTick`
  (params (DeltaSeconds :type "Float (single-precision)"))
  (bind _spawn_point (`self.Spawn Point`))
  (bind _returnvalue (`SceneComponent.K2_GetComponentRotation` _spawn_point))
  (bind _returnvalue_2 (`SceneComponent.K2_GetComponentLocation` _spawn_point))
  ;[0 0.04013 0.23] Shoot player
  (if (`self.isAlive`)
    (if (`self.isMoving`)
      (`KismetSystemLibrary.Delay` 1.5)
      (bind _outhit (`KismetSystemLibrary.LineTraceSingle` :`Start` _returnvalue_2 :`End` (+ _returnvalue_2 (* (`KismetMathLibrary.GetForwardVector` _returnvalue) 500.0)) :`TraceChannel` "TraceTypeQuery1" :`TraceColor` (struct :`R` 1.0 :`G` 0.16921 :`B` 0.998597 :`A` 1.0) :`TraceHitColor` (struct :`R` 0.078316 :`G` 0.146036 :`B` 1.0 :`A` 1.0)))
      ;[1 1 1] VFX
      (`NiagaraFunctionLibrary.SpawnSystemAtLocation` null _returnvalue_2 _returnvalue)
      (cast `/Game/FirstPerson/Blueprints/BP_FirstPersonCharacter` (`GameplayStatics.GetPlayerPawn` (`.ElementIndex` (`GameplayStatics.BreakHitResult` _outhit)))))
    (else
      (`self.K2_DestroyActor`))))

(fn `UserConstructionScript`)