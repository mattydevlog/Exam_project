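; BP_AmmoPickup is an ammo pickup that grants ammo to the player on overlap.
; BeginPlay caches the player character, and the Box overlap event checks the overlapping actor against it.
; A match prints a message, casts to BP_FirstPersonCharacter and calls its AddAmmo.
; The Ammo increment and DestroyActor nodes are disconnected, so this graph leaves the pickup in the world after use.
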(event `self.ReceiveBeginPlay`
  ;[1 1 1] Set player ref
  (set `self.PlayerREF` (`GameplayStatics.GetPlayerCharacter` 0)))

(event `self.Box.OnComponentBeginOverlap`
  (params (OverlappedComponent :type "PrimitiveComponent Object Reference") (OtherActor :type "Actor Object Reference") (OtherComp :type "PrimitiveComponent Object Reference") (OtherBodyIndex :type Integer) (bFromSweep :type Boolean) (SweepResult :type "HitResult Structure (by ref)"))
  ;[0.8566 1 0.3704] Pickup behavior
  (if (== OtherActor (`self.PlayerREF`))
    (`KismetSystemLibrary.PrintString` "Ammo picked up")
    (bind _asbp_first_person_character (cast `/Game/FirstPerson/Blueprints/BP_FirstPersonCharacter` (`GameplayStatics.GetPlayerCharacter` 0)))
    (`/Game/FirstPerson/Blueprints/BP_FirstPersonCharacter.Add ammo` _asbp_first_person_character)))

(fn `UserConstructionScript`)