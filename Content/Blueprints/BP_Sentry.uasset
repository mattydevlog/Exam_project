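; BP_Sentry is an enemy sentry pawn that patrols, turns toward the player and fires line traces to damage them.
; Tick drives movement to the first patrol point and gates shooting on IsMoving, which only disconnected nodes set.
; Pawn sensing starts Delay-looped interpolated facing, gated by a proximity flag.
; Damage decrements HP until Tick destroys the actor; second-patrol and death-effect events are never called here.
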(event `Patrol second`
  (if (`self.hasreachedfirst`)
    (if (not (`self.ShouldRotate`))
      (`/Engine/EditorBlueprintResources/StandardMacros.IsValid` (`self.patrolpoint2`)
        (:`Is Valid`
          (`|AIMoveTo` self (`self.K2_GetActorLocation` (`self.patrolpoint2`)) null))))))

(event `Add index`
  (set `self.CurrentIndexpatrol` (+ (`self.CurrentIndexpatrol`) 1)))

(event `Patrol`
  (bind _patrolpoint (`self.patrolpoint`))
  (if (not (`self.hasreachedfirst`))
    ;[1 1 1] Initial
    (if (not (`self.ShouldRotate`))
      (`/Engine/EditorBlueprintResources/StandardMacros.IsValid` _patrolpoint
        (:`Is Valid`
          (`|AIMoveTo` self (`self.K2_GetActorLocation` _patrolpoint) null))))))

(event `ShouldAIRotate`
  ;[1 1 1] ShouldFaceplayer
  (if (<= (`self.GetDistanceTo` (`GameplayStatics.GetPlayerCharacter` 0) null) 500.0)
    (set `self.ShouldRotate` true)
    (else
      (set `self.ShouldRotate` false)
      (`KismetSystemLibrary.Delay` 0.0001)
      (`self.ShouldAIRotate`))))

(event `RotateTowards`
  (bind (_returnvalue_roll _returnvalue_pitch _returnvalue_yaw) (`KismetMathLibrary.BreakRotator` (`KismetMathLibrary.RInterpTo` (`self.K2_GetActorRotation`) (`KismetMathLibrary.FindLookAtRotation` (`self.K2_GetActorLocation`) (`self.K2_GetActorLocation` (`GameplayStatics.GetPlayerCharacter` 0))) (`GameplayStatics.GetWorldDeltaSeconds`) 20.0)))
  ;[1 1 1] Faceplayer rotation
  (if (`self.ShouldRotate`)
    (`self.K2_SetActorRotation` (`KismetMathLibrary.MakeRotator` _returnvalue_roll _returnvalue_pitch _returnvalue_yaw))
    (`KismetSystemLibrary.Delay` 0.001)
    (`self.RotateTowards`)
    (else
      (`self.ShouldAIRotate`))))

(event `self.ReceiveBeginPlay`
  ;[1 1 1] Set AI movementspeed on start
  (set `FloatingPawnMovement.MaxSpeed` 250.0 (`self.FloatingPawnMovement`)))

(event `self.PawnSensing.OnSeePawn`
  (params (Pawn :type "Pawn Object Reference"))
  ;[1 0.1593 0.9455] AI movement
  (cast `/Game/FirstPerson/Blueprints/BP_FirstPersonCharacter` (`GameplayStatics.GetPlayerCharacter` 0))
  (`self.RotateTowards`))

(event `self.ReceiveAnyDamage`
  (params (Damage :type "Float (single-precision)") (DamageType :type "DamageType Object Reference") (InstigatedBy :type "Controller Object Reference") (DamageCauser :type "Actor Object Reference"))
  ;[0.3545 1 0.2159] Taking damage
  (set `self.isHit` true)
  (if (`self.isAlive`)
    (bind _output_get (set `self.HP1` (- (`self.HP1`) 1.0)))
    (if (<= _output_get 0.0)
      (set `self.isAlive` false))))

(event `Damage VFX`
  ;[1 1 1] VFX damage on player attack
  (`NiagaraFunctionLibrary.SpawnSystemAtLocation` null (`SceneComponent.K2_GetComponentLocation` (`self.Sphere`))))

(event `TakeDamage`)

(event `Death`
  ;[0.04746 1 0.9103] Death state
  (if (not (`self.isAlive`))
    (`GameplayStatics.SpawnEmitterAtLocation` null (`SceneComponent.K2_GetComponentLocation` (`self.Sphere`)))
    (`self.K2_DestroyActor`)))

(event `self.ReceiveTick`
  (params (DeltaSeconds :type "Float (single-precision)"))
  (bind _spawn_point (`self.Spawn Point`))
  (bind _returnvalue (`SceneComponent.K2_GetComponentLocation` _spawn_point))
  ;[0 0.04013 0.23] Shoot player
  (if (not (`self.hasreachedfirst`))
    (`self.Patrol`))
  (if (`self.isAlive`)
    (if (`self.isMoving`)
      (`self.RotateTowards`)
      (`KismetSystemLibrary.Delay` 1.0)
      (bind _outhit (`KismetSystemLibrary.LineTraceSingle` :`Start` _returnvalue :`End` (+ _returnvalue (* (`KismetMathLibrary.GetForwardVector` (`SceneComponent.K2_GetComponentRotation` _spawn_point)) 2500.0)) :`TraceChannel` "TraceTypeQuery1" :`DrawDebugType` "ForDuration" :`TraceColor` (struct :`R` 1.0 :`G` 0.009454 :`A` 1.0) :`TraceHitColor` (struct :`R` 0.078316 :`G` 0.146036 :`B` 1.0 :`A` 1.0)))
      (bind _asbp_first_person_character (cast `/Game/FirstPerson/Blueprints/BP_FirstPersonCharacter` (`.HitActor` (`GameplayStatics.BreakHitResult` _outhit))))
      (`/Game/FirstPerson/Blueprints/BP_FirstPersonCharacter.Take damage` _asbp_first_person_character))
    (else
      (`self.K2_DestroyActor`))))

(fn `UserConstructionScript`)